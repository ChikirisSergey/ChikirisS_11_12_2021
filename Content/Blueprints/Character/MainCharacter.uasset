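; MainCharacter is a player character Blueprint that handles movement, look, sprint and interact input.
; Movement axes add input along the actor's forward and right vectors, LookUp drives controller pitch, and Sprint switches max walk speed while held.
; Interact only prints debug text on press and release.
; Turn is wired into the forward movement node, leaving the controller yaw node unconnected, so it never yaws the view.
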(event `InputAxis|MoveForward`
  (params (AxisValue :type "Float (single-precision)"))
  ;[1 0.2622 0.6378] Входные данные
  ;;[1 1 1] Передвижение
  (`self.AddMovementInput` (`self.GetActorForwardVector`) AxisValue :!label _label))

(event `InputAxis|Moveright`
  (params (AxisValue :type "Float (single-precision)"))
  ;[1 0.2622 0.6378] Входные данные
  ;;[1 1 1] Передвижение
  (`self.AddMovementInput` (`self.GetActorRightVector`) AxisValue))

(event `InputAction|Interact`
  (params (Key :type "Key Structure"))
  ;[1 0.2622 0.6378] Входные данные
  ;;[1 1 1] Взаимодействие
  (:`Pressed`
    (`KismetSystemLibrary.PrintString` "Press"))
  (:`Released`
    (`KismetSystemLibrary.PrintString` "Realese")))

(event `InputAxis|Turn`
  (params (AxisValue :type "Float (single-precision)"))
  ;[1 0.2622 0.6378] Входные данные
  ;;[1 1 1] Поворот
  (goto _label))

(event `InputAxis|LookUp`
  (params (AxisValue :type "Float (single-precision)"))
  ;[1 0.2622 0.6378] Входные данные
  ;;[1 1 1] Поворот
  (`self.AddControllerPitchInput` AxisValue))

(event `InputAction|Sprint`
  (params (Key :type "Key Structure"))
  ;[1 0.2622 0.6378] Входные данные
  ;;[1 1 1] Sprint
  (:`Pressed`
    (set `CharacterMovementComponent.MaxWalkSpeed` 800.0 (`self.CharacterMovement`)))
  (:`Released`
    (set `CharacterMovementComponent.MaxWalkSpeed` 500.0 (`self.CharacterMovement`))))

(fn `UserConstructionScript`)