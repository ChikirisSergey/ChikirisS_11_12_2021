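; Fan actor, judging by its name and folder, that spins four static mesh components until something overlaps its sphere.
; Each tick adds a relative rotation scaled by a speed variable, without delta time, so spin rate follows frame rate.
; Sphere overlap sets OnRotate, which despite its name halts the spin, and any end overlap clears it.
; The Switchlight function and construction script are empty.
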(event `self.ReceiveTick`
  (params (DeltaSeconds :type "Float (single-precision)"))
  (if (not (`self.OnRotate`))
    (`SceneComponent.K2_AddRelativeRotation` (`self.StaticMesh`) (* (`self.Rotation`) (`self.Roration Speed`)) false false)
    (`SceneComponent.K2_AddRelativeRotation` (`self.-StaticMesh2`) (* (`self.Rotation`) (`self.Roration Speed`)) false false)
    (`SceneComponent.K2_AddRelativeRotation` (`self.-StaticMesh4`) (* (`self.Rotation`) (`self.Roration Speed`)) false false)
    (`SceneComponent.K2_AddRelativeRotation` (`self.StaticMesh3`) (* (`self.Rotation`) (`self.Roration Speed`)) false false)))

(event `self.Sphere.OnComponentBeginOverlap`
  (params (OverlappedComponent :type "PrimitiveComponent Object Reference") (OtherActor :type "Actor Object Reference") (OtherComp :type "PrimitiveComponent Object Reference") (OtherBodyIndex :type Integer) (bFromSweep :type Boolean) (SweepResult :type "HitResult Structure (by ref)"))
  (set `self.OnRotate` true))

(event `self.Sphere.OnComponentEndOverlap`
  (params (OverlappedComponent :type "PrimitiveComponent Object Reference") (OtherActor :type "Actor Object Reference") (OtherComp :type "PrimitiveComponent Object Reference") (OtherBodyIndex :type Integer))
  (set `self.OnRotate` false))

(fn `Switchlight`)

(fn `UserConstructionScript`)