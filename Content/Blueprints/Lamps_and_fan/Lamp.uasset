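; Lamp Blueprint that blinks its point light on and off in an endless loop from BeginPlay.
; After a random delay of a few seconds it turns the light on, holds it for a fixed time, then turns it off.
; The Repeat event re-enters the delay chain to restart the cycle, and a SwitchLight helper sets the light's intensity.
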(event `self.ReceiveBeginPlay`
  (`KismetSystemLibrary.Delay` (`KismetMathLibrary.RandomFloatInRange` 1.0 3.0) :!label _label)
  (`self.SwitchLight` 2000.0)
  (`KismetSystemLibrary.Delay` 2.0)
  (`self.SwitchLight` 0.0)
  (`self.Repeat`))

(event `Repeat`
  (goto _label))

(fn `SwitchLight`
  (params (Intensity :type "Float (double-precision)"))
  (`LightComponent.SetIntensity` (`self.PointLight`) Intensity)
  (return))

(fn `UserConstructionScript`)